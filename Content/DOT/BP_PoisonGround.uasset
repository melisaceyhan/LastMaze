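; BP_PoisonGround is a hazard area that deals damage over time to actors standing inside its box.
; Box overlaps maintain a list of actors, adding only those with a BP_HealthComponent and removing them on exit.
; A looping timer applies base damage to every listed actor at a fixed interval.
; It binds to a deactivate-poison event on BP_GameMode2, which destroys the actor when triggered.
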(event OnComponentBeginOverlap(Box)
  (params (OverlappedComponent :type Primitive%20Component%20Object%20Reference) (OtherActor :type Actor%20Object%20Reference) (OtherComp :type Primitive%20Component%20Object%20Reference) (OtherBodyIndex :type Integer) (bFromSweep :type Boolean) (SweepResult :type Hit%20Result%20Structure%20%28by%20ref%29))
  (Utilities|IsValid (Actor|GetComponentbyClass OtherActor "/Game/DOT/BP_HealthComponent.BP_HealthComponent_C")
    (:Is%20Valid
      (Utilities|Array|Add (Variables|Default|GetActorsToDamage) OtherActor))))

(event OnComponentEndOverlap(Box)
  (params (OverlappedComponent :type Primitive%20Component%20Object%20Reference) (OtherActor :type Actor%20Object%20Reference) (OtherComp :type Primitive%20Component%20Object%20Reference) (OtherBodyIndex :type Integer))
  (bind _actorstodamage (Variables|Default|GetActorsToDamage))
  (bind _returnvalue (Utilities|Array|FindItem _actorstodamage OtherActor))
  (if true
    (if (>= _returnvalue 0)
      (Utilities|Array|RemoveIndex (Variables|Default|GetActorsToDamage) _returnvalue))))

(event Custom|DamageTick
  (for _array_element (Variables|Default|GetActorsToDamage)
    (Game|Damage|ApplyDamage _array_element (Variables|Default|GetBaseDamage) 0 0)))

(event Custom|Deactivate
  (Variables|Default|SetActivated false)
  (Actor|DestroyActor))

(event EventBeginPlay
  (bind _asbp_game_mode_2 (Utilities|Casting|CastToBP_GameMode2 (Game|GetGameMode)))
  (EventDispatchers|BindEventtoDeactivatePoision _asbp_game_mode_2 (delegate Custom|Deactivate))
  (Utilities|Time|SetTimerbyEvent (delegate Custom|DamageTick) 0.5 true))

(fn ConstructionScript)