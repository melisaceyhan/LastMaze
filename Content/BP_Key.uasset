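; BP_Key is an interactable key pickup that records its key number in BP_GameMode2.
; BeginPlay caches the game mode, and Interact assigns KeyNumber to its Keys variable, overwriting the previous value.
; It then prints an acquired message using the name looked up from Names and destroys itself.
; The construction script applies the Material variable to the static mesh.
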(event EventInteract
  (bind _output_get (Variables|/Game/Blueprints/BP_GameMode2.BP_GameMode2_C|SetKeys (Variables|Default|GetAs%20BP%20Game%20Mode%202) (Variables|Default|GetKeyNumber)))
  (Development|PrintString (Utilities|String|Append "Key" (Utilities|Array|Get(acopy) (Variables|Default|GetNames) _output_get) "Acquired"))
  (Actor|DestroyActor))

(event EventBeginPlay
  (bind _asbp_game_mode_2 (Utilities|Casting|CastToBP_GameMode2 (Game|GetGameMode)))
  (Variables|Default|SetAs%20BP%20Game%20Mode%202 _asbp_game_mode_2))

(fn ConstructionScript
  (Rendering|Material|SetMaterial (Variables|Default|GetStaticMesh) 0 (Variables|Default|GetMaterial)))