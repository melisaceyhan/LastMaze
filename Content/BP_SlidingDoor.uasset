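; BP_SlidingDoor is an interactable door that slides open when the key value in BP_GameMode2 equals its KeyNumber.
; BeginPlay caches the game mode, and Interact either plays the Door_Rotate timeline or prints a wrong-key message.
; The timeline lerps the Door component's relative location from StartLocation to FinishLocation, with no reverse path to close it.
; The construction script applies a configurable material to the door.
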(event EventBeginPlay
  (bind _asbp_game_mode_2 (Utilities|Casting|CastToBP_GameMode2 (Game|GetGameMode)))
  (Variables|Default|SetAs%20BP%20Game%20Mode%202 _asbp_game_mode_2))

(event EventInteract
  (if (== (Variables|/Game/Blueprints/BP_GameMode2.BP_GameMode2_C|GetKeys (Variables|Default|GetAs%20BP%20Game%20Mode%202)) (Variables|Default|GetKey%20Number))
    (bind _newtrack_0 (Timeline|Door_Rotate Play)
      (:Update
        (Transformation|SetRelativeLocation (Variables|Default|GetDoor) (Math|Vector|Lerp(Vector) (Variables|Default|GetStartLocation) (Variables|Default|GetFinishLocation) _newtrack_0) false false)))
    (else
      (Development|PrintString "You do not have the correct key."))))

(fn ConstructionScript
  (Rendering|Material|SetMaterial (Variables|Default|GetDoor) 0 (Variables|Default|GetMaterial)))