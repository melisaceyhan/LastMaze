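; Maze cell actor that builds one grid square of a maze with optional walls, ceiling and point light.
; The construction script sizes the floor and adds each enabled piece as scaled meshes from grid size and wall height.
; A positive intensity spawns a centered, floor-level light.
; At BeginPlay it binds to the TPC_Maze player's gate event, recoloring the light to the player's color when IsInside is false.
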(event Custom|MazeGate_Event
  (params (isInside? :type Boolean))
  (bind _point_li_ght (Variables|Default|GetPoint%20Lİght))
  (if (not isInside?)
    (Utilities|IsValid _point_li_ght
      (:Is%20Valid
        (Rendering|Components|Light|SetLightColor _point_li_ght (Variables|/Game/TPC_Maze.TPC_Maze_C|GetLightColor (Variables|Default|GetAs%20TPC%20Maze)) true)))))

(event EventBeginPlay
  (bind _astpc_maze (Utilities|Casting|CastToTPC_Maze (Game|Player|GetPlayerPawn 0)))
  (Variables|Default|SetAs%20TPC%20Maze _astpc_maze)
  (EventDispatchers|BindEventtoMazeGate _astpc_maze (delegate Custom|MazeGate_Event)))

(fn ConstructionScript
  (bind _gridsize (Variables|Default|GetGridSize))
  (LocalVariables|SetWallLength _gridsize)
  (LocalVariables|SetWall%20Thickness (* _gridsize 0.1))
  (Transformation|SetRelativeScale3D (Variables|Default|GetFloor) (Utilities|SizetoCubeScale (Math|Vector|MakeVector (LocalVariables|GetWallLength) (LocalVariables|GetWallLength) (LocalVariables|GetWall%20Thickness))))
  (if (Variables|Default|GetWestWall)
    (AddComponent|AddStaticMeshComponent false (Math|Transform|MakeTransform (Math|Vector|MakeVector 0.0 0.0 0.0) "0, 0, 0" (Utilities|SizetoCubeScale (Math|Vector|MakeVector (LocalVariables|GetWallLength) (LocalVariables|GetWall%20Thickness) (Variables|Default|GetWallHeight))))))
  (if (Variables|Default|GetSouthWall)
    (AddComponent|AddStaticMeshComponent false (Math|Transform|MakeTransform (Math|Vector|MakeVector 0.0 0.0 0.0) "0, 0, 0" (Utilities|SizetoCubeScale (Math|Vector|MakeVector (LocalVariables|GetWall%20Thickness) (LocalVariables|GetWallLength) (Variables|Default|GetWallHeight))))))
  (if (Variables|Default|GetNorthWall)
    (AddComponent|AddStaticMeshComponent false (Math|Transform|MakeTransform (Math|Vector|MakeVector (- (LocalVariables|GetWallLength) (LocalVariables|GetWall%20Thickness)) 0.0 0.0) "0, 0, 0" (Utilities|SizetoCubeScale (Math|Vector|MakeVector (LocalVariables|GetWall%20Thickness) (LocalVariables|GetWallLength) (Variables|Default|GetWallHeight))))))
  (if (Variables|Default|GetEastWall)
    (AddComponent|AddStaticMeshComponent false (Math|Transform|MakeTransform (Math|Vector|MakeVector 0.0 (- (LocalVariables|GetWallLength) (LocalVariables|GetWall%20Thickness)) 0.0) "0, 0, 0" (Utilities|SizetoCubeScale (Math|Vector|MakeVector (LocalVariables|GetWallLength) (LocalVariables|GetWall%20Thickness) (Variables|Default|GetWallHeight))))))
  (if (Variables|Default|GetCeiling)
    (AddComponent|AddStaticMeshComponent false (Math|Transform|MakeTransform (Math|Vector|MakeVector 0.0 0.0 (Variables|Default|GetWallHeight)) "0, 0, 0" (Utilities|SizetoCubeScale (Math|Vector|MakeVector (LocalVariables|GetWallLength) (LocalVariables|GetWallLength) (LocalVariables|GetWall%20Thickness))))))
  (if (> (Variables|Default|GetLightIntensity) 0.0)
    (bind _returnvalue (AddComponent|AddPointLightComponent false (Math|Transform|MakeTransform (Math|Vector|MakeVector (* (LocalVariables|GetWallLength) 0.5) (* (LocalVariables|GetWallLength) 0.5) (* 0.0 (Variables|Default|GetWallHeight))) "0, 0, 0" "1.000000,1.000000,1.000000")))
    (bind _output_get (Variables|Default|SetPoint%20Lİght _returnvalue))
    (Rendering|Components|Light|SetIntensity _output_get (Variables|Default|GetLightIntensity))
    (Rendering|Components|Light|SetLightColor _output_get (Variables|Default|GetLightColor) true)))